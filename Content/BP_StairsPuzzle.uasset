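; BP_StairsPuzzle is a stairs actor for a puzzle that rises when its StairsUp event fires, then lowers again.
; BeginPlay stores the starting location and a raised point directly above it.
; StairsUp plays a timer sound and runs a timeline that lerps the actor between the two, reversing once finished.
; A busy flag blocks retriggering during the rise but clears before the descent.
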(event `Stairs Up`
  (if (not (`self.isBusy`))
    (set `self.isBusy` true)
    (`GameplayStatics.PlaySoundAtLocation` "/Game/SoundEffects/TimerNoise.TimerNoise" (stale `self.ReceiveBeginPlay` _output_get_2) (struct) 1.0 1.0 0.0 null null null null)
    (bind (_direction _alpha) (`Timeline|TL_Stairs` :!label _label)
      (:`Update`
        (`self.K2_SetActorLocation` (`KismetMathLibrary.VLerp` (`self.LoweredLocation`) (`self.RaisedLocation`) _alpha)))
      (:`Finished`
        (set `self.isBusy` false)
        (goto _label :!via `Reverse`)))))

(event `self.ReceiveBeginPlay`
  (bind _output_get (set `self.LoweredLocation` (`self.K2_GetActorLocation`)))
  (bind _output_get_2 (set `self.RaisedLocation` (`KismetMathLibrary.MakeVector` (.x _output_get) (.y _output_get) (+ (.z _output_get) 150.0)))))

(fn `UserConstructionScript`)