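; BP_HumanAI is an AI pawn that chases the player and logs its behavior to telemetry.
; PawnSensing sight sets IsSeeingPlayer, logging location on first sighting, and calls FollowPlayer, as does hearing after setting IsHearingPlayer.
; FollowPlayer checks only IsSeeingPlayer, so hearing triggers movement only after a sighting; nothing here clears that flag.
; It uses AIMoveTo and, after a delay, sends both locations as JSON through the GameInstance's TelemetryService.
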(event `self.PawnSensing.OnSeePawn`
  (params (Pawn :type "Pawn Object Reference"))
  ;[1 1 1] when the AI sees the player, call follow player
  (if (`self.IsSeeingPlayer`)
    (`KismetSystemLibrary.PrintString` "i see you")
    (else
      (set `self.IsSeeingPlayer` true) ; make sure Is Seeing Player is set true
      (bind _asmy_game_instance (cast `/Game/Telemetry/MyGameInstance` (`GameplayStatics.GetGameInstance`)))
      (bind _structout (setmembers `JsonObjectWrapper` :`StructRef` (make `JsonObjectWrapper`)))
      (`|SetJsonField` _structout "Location" (`self.K2_GetActorLocation` self))
      (`/Game/Telemetry/TelemetryService.Log Event` (`/Game/Telemetry/MyGameInstance.TelemetryService` _asmy_game_instance) "I see Player" "" _structout)))
  (`self.Follow player`))

(event `Follow player`
  ;[1 1 1] AI Follows the player
  (if (`self.IsSeeingPlayer`)
    (`KismetSystemLibrary.PrintString` "Following")
    (`|AIMoveTo` self (0.0 0.0 0.0) (`GameplayStatics.GetPlayerCharacter` 0) 150.0
      (:`then`
        (`KismetSystemLibrary.Delay` 1.0)
        (bind _asmy_game_instance (cast `/Game/Telemetry/MyGameInstance` (`GameplayStatics.GetGameInstance`)))
        (bind _structout (setmembers `JsonObjectWrapper` :`StructRef` (make `JsonObjectWrapper`)))
        (`|SetJsonField` _structout "Location" (`self.K2_GetActorLocation` self))
        (`|SetJsonField` _structout "Player Location" (`self.K2_GetActorLocation` (`GameplayStatics.GetPlayerCharacter` 0)))
        (`/Game/Telemetry/TelemetryService.Log Event` (`/Game/Telemetry/MyGameInstance.TelemetryService` _asmy_game_instance) "Following Player" "" _structout)))))

(event `self.PawnSensing.OnHearNoise`
  (params (Instigator :type "Pawn Object Reference") (Location :type "Vector Structure (by ref)") (Volume :type "Float (single-precision)"))
  ;[1 1 1] When AI hears Player call FollowPlayer
  (set `self.IsHearingPlayer` true)
  (`self.Follow player`))

(fn `HandleSoundSense`
  (params (Stimulus :type "AIStimulus Structure (by ref)")))

(fn `UserConstructionScript`)