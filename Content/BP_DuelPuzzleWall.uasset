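; BP_DuelPuzzleWall is the door wall for the human and cat double pressure plate puzzle.
; BeginPlay caches its location as closed and derives an open location 300 units higher.
; The DoorOpen event, with no caller in this Blueprint, moves it there instantly, without interpolation.
; It then logs the puzzle as solved, with a JSON payload, through the GameInstance's TelemetryService.
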(event `Door Open`
  (`self.K2_SetActorLocation` (`self.OpenLocation`))
  (bind _asmy_game_instance (cast `/Game/Telemetry/MyGameInstance` (`GameplayStatics.GetGameInstance`)))
  (bind _telemetryservice (`/Game/Telemetry/MyGameInstance.TelemetryService` _asmy_game_instance))
  (`/Game/Telemetry/TelemetryService.Set Section` _telemetryservice "Double Plate Door")
  (bind _structout (setmembers `JsonObjectWrapper` :`StructRef` (make `JsonObjectWrapper`)))
  (`|SetJsonField` _structout "Is Opened" true)
  (`/Game/Telemetry/TelemetryService.Log Event` _telemetryservice "Solved human cat combo plate Puzzle" "" _structout))

(event `self.ReceiveBeginPlay`
  (bind _output_get (set `self.ClosedLocation` (`self.K2_GetActorLocation`)))
  (set `self.OpenLocation` (`KismetMathLibrary.MakeVector` (.x _output_get) (.y _output_get) (+ (.z _output_get) 300.0))))

(fn `UserConstructionScript`)